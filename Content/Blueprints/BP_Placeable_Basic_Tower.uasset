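; Basic placeable tower that automatically fires bullets at a fixed rate while it has health.
; A looping timer spawns BP_Bullet at BulletSpawn and launches it along the Cylinder's up vector, with no target selection.
; ApplyHit deals fixed damage through BPACHealthComponent.
; At zero health the tower stops shooting but stays in place with a death material on its meshes, which Tick also re-applies every frame.
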(event Custom|Shoot
  (if (not (<= (Variables|/Game/Blueprints/Components/BP_AC_HealthComponent.BP_AC_HealthComponent_C|GetHealth (Variables|Default|GetBP_AC_HealthComponent)) 0.0))
    (bind _returnvalue (Game|SpawnActorfromClass "/Game/Blueprints/BP_Bullet.BP_Bullet_C" (Transformation|GetWorldTransform (Variables|Default|GetBulletSpawn)) "Undefined" "MultiplyWithRoot" 0 0))
    (Default|SetUpInitialValues _returnvalue 2e+03 0.5 1.0 (* (Math|Vector|GetUpVector (Transformation|GetWorldRotation (Variables|Default|GetCylinder))) 5e+02) false)))

(event EventBeginPlay
  (Utilities|Time|SetTimerbyEvent (delegate Custom|Shoot) (Variables|Default|GetFireRate) true))

(event EventApplyHit
  (bind _bp_ac_healthcomponent (Variables|Default|GetBP_AC_HealthComponent))
  (bind _deathmat (Variables|Default|GetDeathMat))
  (Default|TakeDamage _bp_ac_healthcomponent 2.0)
  (if (<= (Variables|/Game/Blueprints/Components/BP_AC_HealthComponent.BP_AC_HealthComponent_C|GetHealth _bp_ac_healthcomponent) 0.0)
    (Rendering|Material|SetMaterial (Variables|Default|GetCube) 0 _deathmat)
    (Rendering|Material|SetMaterial (Variables|Default|GetSphere) 0 _deathmat)
    (Rendering|Material|SetMaterial (Variables|Default|GetCylinder) 0 _deathmat)))

(event EventTick
  (params (DeltaSeconds :type Float%20%28single-precision%29))
  (bind _deathmat (Variables|Default|GetDeathMat))
  (if (<= (Variables|/Game/Blueprints/Components/BP_AC_HealthComponent.BP_AC_HealthComponent_C|GetHealth (Variables|Default|GetBP_AC_HealthComponent)) 0.0)
    (Rendering|Material|SetMaterial (Variables|Default|GetCube) 0 _deathmat)
    (Rendering|Material|SetMaterial (Variables|Default|GetSphere) 0 _deathmat)
    (Rendering|Material|SetMaterial (Variables|Default|GetCylinder) 0 _deathmat)))

(fn ConstructionScript
  (|CallParentFunction))