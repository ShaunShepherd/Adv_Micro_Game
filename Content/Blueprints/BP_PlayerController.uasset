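; Player controller Blueprint that sets up Enhanced Input and lets a player request a spawn through a join-game action.
; After a short delay on BeginPlay, it adds the default mapping context to the Enhanced Input local player subsystem if that is valid.
; The join action prints a debug string and calls RestartPlayer on the game mode, with an empty pawn validity check that does not gate the call.
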(event Input|EnhancedActionEvents|EnhancedInputActionIA_JoinGame
  (params (ActionValue :type Boolean) (ElapsedSeconds :type Float%20%28double-precision%29) (TriggeredSeconds :type Float%20%28double-precision%29) (InputAction :type Input%20Action%20Object%20Reference :default "/Game/Input/Actions/IA_JoinGame.IA_JoinGame"))
  (Development|PrintString "Hello")
  (Utilities|IsValid (Pawn|GetControlledPawn)
    (:Is%20Valid
      _)
    (:Is%20Not%20Valid
      _))
  (Class|GameModeBase|RestartPlayer (Game|GetGameMode) self))

(event EventBeginPlay
  (bind _self self)
  (bind _returnvalue (PlayerController|LocalPlayerSubsystems|GetEnhancedInputLocalPlayerSubsystem _self))
  (Utilities|FlowControl|Delay 0.2)
  (Utilities|IsValid _returnvalue
    (:Is%20Valid
      (Input|AddMappingContext _returnvalue "/Game/Input/IMC_Default.IMC_Default" 0 "(bIgnoreAllPressedKeysUntilRelease=True,bForceImmediately=False,bNotifyUserSettings=False)"))))

(fn ConstructionScript)