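; Obstacle placement manager that populates placement points with randomly chosen objects within a cost budget at BeginPlay.
; It shuffles the placement positions and moves a spawned pick to each until no valid pick remains.
; Each pick spawns a random class to read its cost, deducting it from the budget if affordable.
; Otherwise it destroys the spawn and retries after removing a randomly drawn class, not necessarily the rejected one, from a temporary list.
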(event EventBeginPlay
  (bind _placementpositions (Variables|Default|GetPlacementPositions))
  (Utilities|Array|Shuffle _placementpositions)
  (bind _array_element (Utilities|Array|ForEachLoopwithBreak _placementpositions :!label _label)
    (:LoopBody
      (bind _selectedplaceable (CallFunction|PickObjecttoPlace))
      (Utilities|IsValid _selectedplaceable
        (:Is%20Valid
          (Transformation|SetActorTransform _selectedplaceable (Transformation|GetWorldTransform (Variables|/Script/Engine.Actor|GetRootComponent _array_element))))
        (:Is%20Not%20Valid
          (goto _label Break))))))

(fn ConstructionScript)

(fn PickObjecttoPlace
  (bind _placeableobjectstemp (Variables|Default|GetPlaceableObjectsTemp))
  (bind _outitem (Utilities|Array|Random _placeableobjectstemp))
  (|CreateTempArray
    (:Completed
      (bind _returnvalue (Game|SpawnActorfromClass _outitem (Transformation|GetActorTransform) "Undefined" "MultiplyWithRoot" 0 0 :!label _label))
      (if (>= (- (Variables|Default|GetTotalPlacementPoints) (Variables|/Game/Blueprints/BP_Placeable_Obstacle.BP_Placeable_Obstacle_C|GetPlacementCost _returnvalue)) 0.0)
        (Variables|Default|SetTotalPlacementPoints (- (Variables|Default|GetTotalPlacementPoints) (Variables|/Game/Blueprints/BP_Placeable_Obstacle.BP_Placeable_Obstacle_C|GetPlacementCost _returnvalue)))
        (else
          (Utilities|Array|RemoveItem (Variables|Default|GetPlaceableObjectsTemp) _outitem)
          (if (> (Utilities|Array|Length (Variables|Default|GetPlaceableObjectsTemp)) 0)
            (Actor|DestroyActor _returnvalue)
            (goto _label)
            (else
              (Actor|DestroyActor _returnvalue)))))
      (return _returnvalue))))