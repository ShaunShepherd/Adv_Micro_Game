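; BP_Bullet is a projectile, fired by either player or enemy, that damages its target and destroys itself on a hit or beyond its range.
; The spawning weapon initializes material, scale, damage, velocity and range, which enables collision.
; On overlap, the damage component hits BP_Placeable_Basic_Tower actors for player bullets, or BP_PlayerCharacter for enemy bullets.
; ApplyHit deflects the bullet by reversing velocity and making it a player bullet.
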(event OnComponentBeginOverlap(Collider)
  (params (OverlappedComponent :type Primitive%20Component%20Object%20Reference) (OtherActor :type Actor%20Object%20Reference) (OtherComp :type Primitive%20Component%20Object%20Reference) (OtherBodyIndex :type Integer) (bFromSweep :type Boolean) (SweepResult :type Hit%20Result%20Structure%20%28by%20ref%29))
  (if (Variables|Default|GetPlayerBullet)
    (bind _array_element (Utilities|Array|ForEachLoopwithBreak (Collision|GetOverlappingActors (Variables|Default|GetCollider) "/Game/Blueprints/BP_Placeable_Basic_Tower.BP_Placeable_Basic_Tower_C" :!class /Script/Engine.PrimitiveComponent))
      (:LoopBody
        (Default|ApplyDamage (Variables|Default|GetBP_AC_DamageComponent) _array_element)
        (Variables|Default|SetHitSomething true))
      (:Completed
        (if (Variables|Default|GetHitSomething) :!label _label
          (Actor|DestroyActor))))
    (else
      (bind _array_element_2 (Utilities|Array|ForEachLoopwithBreak (Collision|GetOverlappingActors (Variables|Default|GetCollider) "/Game/Blueprints/BP_PlayerCharacter.BP_PlayerCharacter_C" :!class /Script/Engine.PrimitiveComponent))
        (:LoopBody
          (Default|ApplyDamage (Variables|Default|GetBP_AC_DamageComponent) _array_element_2)
          (Variables|Default|SetHitSomething true)
          (Development|PrintString "Hir player"))
        (:Completed
          (goto _label))))))

(event Custom|SetUpInitialValues
  (params (Range :type Float%20%28double-precision%29) (Scale :type Float%20%28double-precision%29) (DamageAmount :type Float%20%28double-precision%29) (Velocity :type Vector) (IsPlayerBullet :type Boolean))
  (bind _sphere (Variables|Default|GetSphere))
  ;[0.15 0.15 0.15 0.5] Called when weapon creates bullet
  (bind _output_get (Variables|Default|SetPlayerBullet IsPlayerBullet))
  (if _output_get
    (Rendering|Material|SetMaterial _sphere 0 (Variables|Default|GetPlayerBulletMat))
    (else
      (Rendering|Material|SetMaterial _sphere 0 (Variables|Default|GetEnemyBulletMat))))
  (Variables|Default|SetRange Range)
  (Variables|Default|SetStartPos (Transformation|GetWorldLocation (Variables|Default|GetSphere)))
  (Transformation|SetWorldScale3D (Variables|Default|GetSphere) (* Scale (Math|Vector|MakeVector 1.0 1.0 1.0)))
  (Variables|/Game/Blueprints/Components/BP_AC_DamageComponent.BP_AC_DamageComponent_C|SetDamageAmount (Variables|Default|GetBP_AC_DamageComponent) DamageAmount)
  (Variables|/Script/Engine.MovementComponent|SetVelocity (Variables|Default|GetProjectileMovement) Velocity)
  (Collision|SetCollisionEnabled (Variables|Default|GetCollider) "QueryAndPhysics"))

(event EventTick
  (params (DeltaSeconds :type Float%20%28single-precision%29))
  ;[0.15 0.15 0.15 0.5] Handle range, delete object once travelled range value
  (if (> (Math|Vector|Distance(Vector) (Variables|Default|GetStartPos) (Transformation|GetWorldLocation (Variables|Default|GetSphere))) (Variables|Default|GetRange))
    (Actor|DestroyActor)))

(event EventBeginPlay
  (Collision|SetCollisionEnabled (Variables|Default|GetCollider) "NoCollision"))

(event EventApplyHit
  (Variables|/Script/Engine.MovementComponent|SetVelocity (Variables|Default|GetProjectileMovement) (* (Variables|/Script/Engine.MovementComponent|GetVelocity (Variables|Default|GetProjectileMovement)) -1.0))
  (Development|PrintString "Bullet hit")
  (Variables|Default|SetPlayerBullet true)
  (Rendering|Material|SetMaterial (Variables|Default|GetSphere) 0 (Variables|Default|GetPlayerBulletMat)))

(fn ConstructionScript)