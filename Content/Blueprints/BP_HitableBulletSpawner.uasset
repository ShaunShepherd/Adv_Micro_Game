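; BP_HitableBulletSpawner is a hittable actor that fires a radial burst of player bullets when hit.
; ApplyHit damages its health component by one and, unless health drops below zero, spawns eight BP_Bullet actors.
; A BulletSpawn component rotates in 45-degree steps to aim each bullet's velocity.
; The hit that brings health to exactly zero turns the sphere blue and still fires a final burst.
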(event EventApplyHit
  (bind _bp_ac_healthcomponent (Variables|Default|GetBP_AC_HealthComponent))
  (bind _health (Variables|/Game/Blueprints/Components/BP_AC_HealthComponent.BP_AC_HealthComponent_C|GetHealth _bp_ac_healthcomponent))
  (Default|TakeDamage _bp_ac_healthcomponent 1.0)
  (if (not (< _health 0.0))
    (if (== _health 0.0)
      (Rendering|Material|SetMaterial (Variables|Default|GetSphere) 0 "/Game/LevelPrototyping/Materials/MI_Solid_Blue.MI_Solid_Blue"))
    (for _index (range 0 7)
      (bind _returnvalue (Game|SpawnActorfromClass "/Game/Blueprints/BP_Bullet.BP_Bullet_C" (Transformation|GetWorldTransform (Variables|Default|GetBulletSpawn)) "Undefined" "MultiplyWithRoot" 0 0))
      (Transformation|SetRelativeRotation (Variables|Default|GetBulletSpawn) (Math|Rotator|MakeRotator 0.0 0.0 (* (Math|Conversions|ToFloat(Integer) _index) 45.0)) false false)
      (Default|SetUpInitialValues _returnvalue 5e+03 0.2 1.0 (* (Math|Vector|GetForwardVector (Transformation|GetWorldRotation (Variables|Default|GetBulletSpawn))) 5e+02) true))))

(fn ConstructionScript)