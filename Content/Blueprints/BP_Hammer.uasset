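; Player hammer that stretches its handle while charged, slams, then pivots about the impact point to swing the player along.
; Chained timelines drive the slam, the player swing with the hammer as parent, and the length reset.
; On impact it shakes the camera, fires Niagara and sphere-traces at the head, messaging BP_I_HammerHit actors.
; Timer-based early and late combo windows allow another swing at the charged length.
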(event Custom|SetPlayerRef
  (params (PlayerRef :type BP%20Player%20Character%20Object%20Reference))
  ;[0.15 0.15 0.15 0.5] Called by Player When Spawned
  (Variables|Default|SetPlayer%20Ref PlayerRef))

(event Custom|ResetHammer
  (Variables|Default|SetPercentageSwung (Variables|Default|GetPercentageHeld))
  (bind _newtrack_0 (Timeline|HammerLengthReset PlayFromStart)
    (:Update
      (bind _output_get (Variables|Default|SetPercentageHeld (Math|Float|Lerp (Variables|Default|GetPercentageSwung) 0.0 _newtrack_0)))
      (CallFunction|SetHammerLength _output_get))
    (:Finished
      (Default|HammerHit (Variables|Default|GetPlayer%20Ref) true)
      (Variables|Default|SetPercentageHeld 0.0)
      (Development|PrintString "finnished"))))

(event Custom|SwingHammer
  (bind _aimdirectionparent (Variables|Default|GetAimDirectionParent))
  (bind _hammerparent (Variables|Default|GetHammerParent))
  (bind _relativelocation (Variables|/Script/Engine.SceneComponent|GetRelativeLocation _hammerparent))
  (bind _relativelocation_2 (Variables|/Script/Engine.SceneComponent|GetRelativeLocation _aimdirectionparent))
  (Variables|Default|SetSwingConsumed true)
  (Variables|Default|SetPercentageSwung 0.0)
  (Variables|Default|SetSwinging true)
  (Default|HammerHit (Variables|Default|GetPlayer%20Ref) false)
  (bind _swingrot (Timeline|HammerSwing PlayFromStart)
    (:Update
      (Transformation|SetRelativeRotation (Variables|Default|GetAimDirectionParent) (Math|Rotator|MakeRotator 0.0 _swingrot 0.0) false false))
    (:Finished
      (Transformation|SetRelativeLocation _aimdirectionparent (Math|Vector|MakeVector (+ (Variables|Default|GetHitLength) (.x _relativelocation_2)) (.y _relativelocation_2) (.z _relativelocation_2)) false true)
      (Transformation|SetRelativeLocation _hammerparent (Math|Vector|MakeVector (+ (Variables|Default|GetHitLength) (.x _relativelocation)) (.y _relativelocation) (.z _relativelocation)) false true)
      (Default|ToggleHammerasParent (Variables|Default|GetPlayer%20Ref) true)
      (Default|ShakeCamera (Variables|Default|GetMainCamRef))
      (Utilities|FlowControl|Delay 0.075)
      (Components|Activation|Activate (Variables|Default|GetNE_HammerHit_System) true)
      (CallFunction|CheckforHits)
      (bind _playermoverot (Timeline|SwingPlayer PlayFromStart)
        (:Update
          (Transformation|SetRelativeRotation (Variables|Default|GetAimDirectionParent) (Math|Rotator|MakeRotator 0.0 _playermoverot 0.0) false false))
        (:Finished
          (Utilities|FlowControl|Delay 0.1)
          (Default|ToggleHammerasParent (Variables|Default|GetPlayer%20Ref) false)
          (Transformation|SetRelativeLocation (Variables|Default|GetAimDirectionParent) "0, 0, 0" false false)
          (Transformation|SetRelativeLocation (Variables|Default|GetHammerParent) "0, 0, 0" false false)
          (if (Variables|Default|GetSwingCombo)
            (CallFunction|SwingHammer)
            (Development|PrintString "Early")
            (else
              (Variables|Default|SetCanLateCombo true)
              (Utilities|Time|SetTimerbyFunctionName 0 "ComboLateDelay" (Variables|Default|GetComboDelayMax))
              (CallFunction|ResetHammer))))))))

(event Custom|StopHammerReset
  (Development|PrintString "stopping")
  (bind _newtrack_0 (Timeline|HammerLengthReset Stop)
    (:Update
      (bind _output_get (Variables|Default|SetPercentageHeld (Math|Float|Lerp (Variables|Default|GetPercentageSwung) 0.0 _newtrack_0)))
      (CallFunction|SetHammerLength _output_get))
    (:Finished
      (Default|HammerHit (Variables|Default|GetPlayer%20Ref) true)
      (Variables|Default|SetPercentageHeld 0.0)
      (Development|PrintString "finnished"))))

(event Custom|SpawnHitCollider)

(event Custom|SlamHammer_Started
  (Variables|Default|SetSwingConsumed false))

(event Custom|SlamHammer_Ongoing
  (params (ElapsedSeconds :type Float%20%28double-precision%29))
  (if (not (Variables|Default|GetSwinging))
    (if (not (Variables|Default|GetSwingConsumed))
      (bind _output_get (Variables|Default|SetPercentageHeld (Math|Float|Clamp(Float) (+ (Variables|Default|GetPercentageHeld) (* ElapsedSeconds (Variables|Default|GetChargeRate))))))
      (CallFunction|SetHammerLength _output_get))))

(event Custom|SlamHammer_Complete
  (if (not (Variables|Default|GetSwingConsumed))
    (if (Variables|Default|GetSwinging)
      (if (Variables|Default|GetCanLateCombo)
        (CallFunction|StopHammerReset)
        (bind _output_get (Variables|Default|SetPercentageHeld (Variables|Default|GetPercentageSwung)))
        (CallFunction|SetHammerLength _output_get)
        (CallFunction|SwingHammer)
        (Variables|Default|SetCanLateCombo false)
        (else
          (Variables|Default|SetSwingCombo true)
          (Utilities|Time|SetTimerbyFunctionName 0 "ComboEarlyDelay" (Variables|Default|GetComboDelayMax))))
      (else
        (CallFunction|SwingHammer)
        (Variables|Default|SetSwingConsumed true)
        (Development|PrintString "Regular Swing")))))

(event EventBeginPlay
  (Utilities|FlowControl|Delay 0.2)
  (bind _asbp_game_state (Utilities|Casting|CastToBP_GameState (Game|GetGameState)))
  (Variables|Default|SetMainCamRef (Variables|/Game/Blueprints/BP_GameState.BP_GameState_C|GetMainCamRef _asbp_game_state)))

(fn ConstructionScript)

(fn SetHammerLength
  (params (PercentageHeld :type Float%20%28double-precision%29))
  (bind _handle (Variables|Default|GetHandle))
  (bind _handle_2 (Variables|Default|GetHandle))
  (bind _minlength (Variables|Default|GetMinLength))
  (bind _weight (Variables|Default|GetWeight))
  (bind _handle_3 (Variables|Default|GetHandle))
  (bind _relativescale3d (Variables|/Script/Engine.SceneComponent|GetRelativeScale3D _handle_3))
  (bind _relativescale3d_2 (Variables|/Script/Engine.SceneComponent|GetRelativeScale3D _handle_2))
  (bind _relativelocation (Variables|/Script/Engine.SceneComponent|GetRelativeLocation _handle))
  (bind _relativelocation_2 (Variables|/Script/Engine.SceneComponent|GetRelativeLocation _weight))
  (bind _returnvalue (* (.z _relativescale3d) 1e+02))
  (Transformation|SetRelativeScale3D (Variables|Default|GetHandle) (Math|Vector|MakeVector (.x _relativescale3d_2) (.y _relativescale3d_2) (+ _minlength (* PercentageHeld (- (Variables|Default|GetMaxLength) _minlength)))))
  (Transformation|SetRelativeLocation (Variables|Default|GetHandle) (Math|Vector|MakeVector (/ (* (.z (Variables|/Script/Engine.SceneComponent|GetRelativeScale3D _handle)) 1e+02) 2.0) (.y _relativelocation) (.z _relativelocation)) false false)
  (Transformation|SetRelativeLocation _weight (Math|Vector|MakeVector _returnvalue (.y _relativelocation_2) (.z _relativelocation_2)) false true)
  (Variables|Default|SetHitLength _returnvalue)
  (return))

(fn ComboEarlyDelay
  (Variables|Default|SetSwingCombo false)
  (Development|PrintString "Combo Ran Out"))

(fn ComboLateDelay
  (Variables|Default|SetSwinging false)
  (Variables|Default|SetCanLateCombo false)
  (Development|PrintString "Late window closed"))

(fn CheckforHits
  (bind _weight (Variables|Default|GetWeight))
  (bind _returnvalue (Transformation|GetWorldLocation _weight))
  (bind _outhits (Collision|MultiSphereTraceByChannel _returnvalue _returnvalue 125.0 "TraceTypeQuery1" false 0 "None"))
  (for _array_element _outhits
    (if (Utilities|DoesObjectImplementInterface (.HitActor (Collision|BreakHitResult _array_element)) "/Game/Blueprints/Interfaces/BP_I_HammerHit.BP_I_HammerHit_C")
      (if (!= (.HitActor (Collision|BreakHitResult _array_element)) (Variables|Default|GetPlayer%20Ref))
        (Class|BPIHammerHit|ApplyHit(Message) (.HitActor (Collision|BreakHitResult _array_element))))))
  (return))