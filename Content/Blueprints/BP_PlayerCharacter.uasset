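; BP_PlayerCharacter is the isometric player character, which spawns and carries a BP_Hammer and gives it a reference back to itself.
; Enhanced Input movement is rotated -45 degrees to suit the camera angle.
; ToggleHammerAsParent swaps the attachment hierarchy so the hammer carries the player, disabling capsule collision and movement input until toggled back.
; HammerHit stores a CanMove flag, which movement input does not check.
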(event Custom|HammerHit
  (params (Finished :type Boolean))
  (Variables|Default|SetCanMove Finished))

(event Custom|ToggleHammerAsParent
  (params (HammerParent :type Boolean))
  (bind _hammerref (Variables|Default|GetHammerRef))
  (bind _output_get (Variables|Default|SetIsNotParent HammerParent))
  (if _output_get
    (Transformation|DetachFromActor (Variables|Default|GetHammerRef) "KeepWorld" "KeepWorld" "KeepWorld")
    (Transformation|AttachComponentToComponent (Variables|/Game/Blueprints/BP_Hammer.BP_Hammer_C|GetHammerParent (Variables|Default|GetHammerRef)) "None" "KeepWorld" "KeepWorld" "KeepWorld" true)
    (Collision|SetCollisionEnabled (Variables|Default|GetCapsuleComponent) "NoCollision")
    (else
      (Transformation|DetachFromActor "KeepWorld" "KeepWorld" "KeepWorld")
      (Transformation|AttachActorToActor _hammerref self "None" "KeepWorld" "KeepWorld" "KeepWorld" true)
      (Transformation|SetActorLocation _hammerref (Transformation|GetWorldLocation (Variables|Default|GetHammerHoldPos)) false false)
      (Collision|SetCollisionEnabled (Variables|Default|GetCapsuleComponent) "QueryAndPhysics"))))

(event Input|EnhancedActionEvents|EnhancedInputActionIA_Move
  (params (ActionValue :type Vector%202D%20Structure) (ElapsedSeconds :type Float%20%28double-precision%29) (TriggeredSeconds :type Float%20%28double-precision%29) (InputAction :type Input%20Action%20Object%20Reference :default "/Game/Input/Actions/IA_Move.IA_Move"))
  (bind _returnvalue (Pawn|GetControlRotation :!class /Script/Engine.Pawn))
  ;[0.15 0.15 0.15 0.5] Handle movement input
  (if (not (Variables|Default|GetIsNotParent))
    (Pawn|Input|AddMovementInput (Math|Vector|RotateVectorAroundAxis (Math|Vector|GetRightVector (Math|Rotator|MakeRotator (.roll _returnvalue) 0.0 (.yaw _returnvalue))) -45.0 "0.000000,0.000000,1.000000") (.x ActionValue) false)
    (Pawn|Input|AddMovementInput (Math|Vector|RotateVectorAroundAxis (Math|Vector|GetForwardVector (Math|Rotator|MakeRotator 0.0 0.0 (.yaw (Pawn|GetControlRotation :!class /Script/Engine.Pawn)))) -45.0 "0.000000,0.000000,1.000000") (.y ActionValue) false)))

(event EventBeginPlay
  (bind _self self)
  (bind _returnvalue (Game|SpawnActorfromClass "/Game/Blueprints/BP_Hammer.BP_Hammer_C" (Math|Transform|MakeTransform (Variables|/Script/Engine.SceneComponent|GetRelativeLocation (Variables|Default|GetHammerHoldPos)) "0, 0, 0" "1.000000,1.000000,1.000000") "Undefined" "MultiplyWithRoot" 0 0))
  (bind _output_get (Variables|Default|SetHammerRef _returnvalue))
  (Default|SetPlayerRef _output_get _self)
  (Transformation|AttachActorToActor _returnvalue _self "None" "KeepRelative" "KeepRelative" "KeepRelative" true))

(event EventControllerChanged
  (params (OldController :type Controller%20Object%20Reference) (NewController :type Controller%20Object%20Reference))
  ;[0.15 0.15 0.15 0.5] Configure input map
  (bind _asplayer_controller (Utilities|Casting|CastToPlayerController NewController))
  (Input|AddMappingContext (PlayerController|LocalPlayerSubsystems|GetEnhancedInputLocalPlayerSubsystem _asplayer_controller) "/Game/Input/IMC_Default.IMC_Default" 0 "(bIgnoreAllPressedKeysUntilRelease=True,bForceImmediately=False,bNotifyUserSettings=False)"))

(fn ConstructionScript)