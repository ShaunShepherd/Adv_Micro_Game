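; BP_GameState tracks how many things have been destroyed and triggers the win condition for a destruction-based game.
; Each IncreaseDestroyedThings call increments the counter and compares it to ThingsDestroyedToWin.
; Reaching the threshold shows the BP_W_GameWinScreen widget, pauses the game and switches the first player to UI-only input with a visible cursor.
; Calls below the threshold only print a "SMASH SMASH" message.
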(event Custom|IncreaseDestroyedThings
  (bind _returnvalue (Game|GetPlayerController 0))
  (bind _result (Math|Integer|IncrementInt (Variables|Default|GetCurrentAmountOfThingsDestroyed))
    (:%20%20
      (if (>= _result (Variables|Default|GetThingsDestroyedToWin))
        (bind _returnvalue_2 (UserInterface|CreateWidget "/Game/Menus/BP_W_GameWinScreen.BP_W_GameWinScreen_C"))
        (UserInterface|Viewport|AddtoViewport _returnvalue_2 0)
        (Game|SetGamePaused true)
        (Input|SetInputModeUIOnly _returnvalue 0 "DoNotLock" false)
        (Variables|/Script/Engine.PlayerController|SetbShowMouseCursor _returnvalue true)
        (else
          (Development|PrintString "SMASH SMASH"))))))

(fn ConstructionScript)